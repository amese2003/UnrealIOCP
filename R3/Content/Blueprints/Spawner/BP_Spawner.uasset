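; Spawner Blueprint that creates monster actors from a creature ID at a given location and rotation.
; BeginPlay starts an async load of MonsterTable, but the loaded result is not used in this graph.
; SpawnMonster looks up the actor class in the MonsterTableAct map, spawns it and registers valid actors under their ObjectId.
; A data table row lookup on MonsterTable is left unconnected.
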(event EventBeginPlay
  (Utilities|AsyncLoadAsset (Utilities|ResolveSoftReference (Variables|Default|GetMonsterTable))))

(event Collision|EventActorBeginOverlap
  (params (OtherActor :type Actor%20Object%20Reference)))

(event EventTick
  (params (DeltaSeconds :type Float%20%28single-precision%29)))

(event EventSpawnMonster
  (params (object_id :type Integer) (CreatureID :type Integer) (Location :type Vector :default "0, 0, 0") (Rotator :type Rotator :default "0, 0, 0") (speed :type Float%20%28single-precision%29))
  (bind _monstertable_act (Variables|Default|GetMonsterTable_act))
  (bind (_value _returnvalue) (Utilities|Map|Find _monstertable_act CreatureID))
  (if _returnvalue
    (bind _returnvalue_2 (Game|SpawnActorfromClass _value (Math|Transform|MakeTransform Location Rotator) "Undefined" "MultiplyWithRoot" 0 0))
    (Utilities|IsValid _returnvalue_2
      (:Is%20Valid
        (Class|R3Spawner|RegisterMonsterActor object_id _returnvalue_2)))))

(fn ConstructionScript)