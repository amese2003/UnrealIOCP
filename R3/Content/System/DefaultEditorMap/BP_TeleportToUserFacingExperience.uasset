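; Teleporter actor that sends a local player into a configured user-facing experience when their pawn overlaps it.
; On BeginPlay it async-loads the experience's map primary asset and shows that asset's display name on a text render.
; Overlap by a locally controlled pawn builds a hosting request from the experience and passes it to CommonSessionSubsystem's HostSession to start the session.
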(event Custom|LoadingIntoExperience
  (params (ForPlayer :type Player%20Controller%20Object%20Reference))
  (Utilities|IsValid (Variables|Default|GetUserFacingExperienceToLoad)
    (:Is%20Valid
      (bind _returnvalue (Class|R3UserFacingExperienceDefinition|CreateHostingRequest (Variables|Default|GetUserFacingExperienceToLoad)))
      (Class|CommonSessionSubsystem|HostSession (Subsystems|GetCommonSessionSubsystem) ForPlayer _returnvalue))))

(event EventBeginPlay
  (bind _loaded (|AsyncLoadPrimaryAsset (Variables|/Script/R3.R3UserFacingExperienceDefinition|GetMapID (Variables|Default|GetUserFacingExperienceToLoad)))
    (:Completed
      (Rendering|Components|TextRender|SetText (Variables|Default|GetTextRender) (Utilities|Text|ToText(String) (Utilities|GetDisplayName _loaded))))))

(event Collision|EventActorBeginOverlap
  (params (OtherActor :type Actor%20Object%20Reference))
  (bind _as폰 (Utilities|Casting|CastToPawn OtherActor))
  (Utilities|IsValid (Pawn|GetController _as폰)
    (:Is%20Valid
      (if (Pawn|IsLocalController (Pawn|GetController _as폰))
        (CallFunction|LoadingIntoExperience (.As플레이어%20컨트롤러 (Utilities|Casting|CastToPlayerController (Pawn|GetController _as폰))))))))

(event EventTick
  (params (DeltaSeconds :type Float%20%28single-precision%29)))

(fn ConstructionScript)